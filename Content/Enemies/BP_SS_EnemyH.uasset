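; Enemy H child Blueprint that starts with its movement vector along its right axis and reacts to side boundaries.
; Overlapping an actor tagged "Lateral" toggles IsRight, and each switch away from right also shortens DelayShoot.
; Both branches set MovementVector to the negated right vector, so the else branch does not restore rightward movement.
; Tick is disabled, and this Blueprint only sets these variables without moving or shooting itself.
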(event EventBeginPlay
  (|CallParentFunction)
  (Variables|Default|SetMovementVector (Transformation|GetActorRightVector))
  (Variables|Default|SetIsRight true))

(event Collision|EventActorBeginOverlap
  (params (OtherActor :type Actor%20Object%20Reference))
  (bind _returnvalue (Transformation|GetActorRightVector))
  (bind _returnvalue_2 (* _returnvalue -1.0))
  (|CallParentFunction OtherActor)
  (if (Utilities|Array|ContainsItem (Variables|/Script/Engine.Actor|GetTags OtherActor) "Lateral")
    (if (Variables|Default|GetIsRight)
      (Variables|Default|SetIsRight false)
      (Variables|Default|SetMovementVector _returnvalue_2)
      (Variables|Default|SetDelayShoot (- (Variables|Default|GetDelayShoot) 0.1))
      (else
        (Variables|Default|SetIsRight true)
        (Variables|Default|SetMovementVector _returnvalue_2)))))

(event EventTick
  (params (DeltaSeconds :type Float%20%28single-precision%29))
  (|CallParentFunction DeltaSeconds) ; Este nodo está deshabilitado y no se le llamará.\nArrastra pines para construir una funcionalidad.
)

(fn ConstructionScript
  (|CallParentFunction))